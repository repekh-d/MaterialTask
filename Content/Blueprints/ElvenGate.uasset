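; Elven gate actor whose hidden text shows only when the player pawn stands within a certain angle of it.
; BeginPlay creates a dynamic material for HiddenText, and Tick drives its Visibility parameter from AttenuateBasedOnAngle.
; That function compares horizontally projected text-forward and actor-to-pawn directions by cosine, peaking mid-range and fading to zero toward both angle limits.
; A distance-based attenuation function is also defined but unused.
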(event `self.ReceiveBeginPlay`
  (bind _returnvalue (`PrimitiveComponent.CreateDynamicMaterialInstance` (`self.HiddenText`) 0 "/Game/Materials/TextMaterial.TextMaterial" "None"))
  (set `self.TextMaterial` _returnvalue))

(event `self.ReceiveTick`
  (params (DeltaSeconds :type "Float (single-precision)"))
  (bind _factor (`self.AttenuateBasedOnAngle` 30.0 60.0))
  (`MaterialInstanceDynamic.SetScalarParameterValue` (`self.TextMaterial`) "Visibility" _factor))

(fn `AttenuateBasedOnAngle`
  (params (MinAngle :type "Float (double-precision)") (MaxAngle :type "Float (double-precision)"))
  (returns (Factor :type "Float (double-precision)"))
  (bind _returnvalue (`KismetMathLibrary.DegCos` MinAngle))
  (bind _returnvalue_2 (`KismetMathLibrary.DegCos` MaxAngle))
  (bind _returnvalue_3 (/ (+ _returnvalue _returnvalue_2) 2.0))
  (bind _returnvalue_4 (`KismetMathLibrary.Vector_CosineAngle2D` (`KismetMathLibrary.Normal` (`KismetMathLibrary.ProjectVectorOnToPlane` (`KismetMathLibrary.GetDirectionUnitVector` (`self.K2_GetActorLocation`) (`self.K2_GetActorLocation` (`GameplayStatics.GetPlayerPawn` 0))) (0.0 0.0 1.0))) (`KismetMathLibrary.Normal` (`KismetMathLibrary.ProjectVectorOnToPlane` (`SceneComponent.GetForwardVector` (`self.HiddenText`)) (0.0 0.0 1.0)))))
  ;[1 1 1] Clamp and map to [0, 1] with 1 in the middle of the range
  (if (< _returnvalue_4 _returnvalue_3)
    (return (`KismetMathLibrary.MapRangeClamped` _returnvalue_4 _returnvalue_2 _returnvalue_3 0.0 1.0))
    (else
      (return (`KismetMathLibrary.MapRangeClamped` _returnvalue_4 _returnvalue_3 _returnvalue 1.0)))))

(fn `AttenuateBasedOnDistance`
  (params (MinDistance :type "Float (double-precision)") (MaxDistance :type "Float (double-precision)"))
  (returns (Coeficient :type "Float (double-precision)"))
  (return (`KismetMathLibrary.MapRangeClamped` (`KismetMathLibrary.Vector_Distance` (`self.K2_GetActorLocation`) (`self.K2_GetActorLocation` (`GameplayStatics.GetPlayerPawn` 0))) MinDistance MaxDistance 1.0)))

(fn `UserConstructionScript`)